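; Example game state for the XD camp (faction) system that sets up the game's starting camps.
; On WhenGameInit it adds two camps, named 阵营1 and 阵营2 ("Camp 1" and "Camp 2"), to its XDCampManager.
; It exposes that manager through GetCampManager and returns false from NeedNotSave, so it does not opt out of saving.
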(event `self.ReceiveBeginPlay`)

(event `XD_SaveGameInterface.WhenGameInit`
  (`XD_CampManager.AddCamp` (`self.XD_CampManager`) "阵营1")
  (`XD_CampManager.AddCamp` (`self.XD_CampManager`) "阵营2"))

(fn `GetCampManager`
  (returns (ReturnValue :type "XD_CampManager Object Reference"))
  (return (`self.XD_CampManager`)))

(fn `NeedNotSave`
  (returns (ReturnValue :type Boolean))
  (return false))

(fn `UserConstructionScript`)